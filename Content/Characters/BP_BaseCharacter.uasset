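; BP_BaseCharacter is a character Blueprint that adds debug hotkeys for testing the game's save and load system.
; K and L call the global save and load functions, while Y and U call the local, slot-based versions on slot 0.
; Each key prints an on-screen confirmation after its call.
; The save functions are defined outside this graph, and BeginPlay, Tick, overlap and construction logic are empty.
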(event EventBeginPlay)

(event Collision|EventActorBeginOverlap
  (params (OtherActor :type Actor%20Object%20Reference)))

(event EventTick
  (params (DeltaSeconds :type Float%20%28single-precision%29)))

(event Input|KeyboardEvents|DebugKeyY
  (params (Key :type Key%20Structure :default "None") (ActionValue :type Input%20Action%20Value%20Structure))
  (:Pressed
    (Class|BaseCharacter|SaveGameLocally)
    (Development|PrintString "Saved Slot 0")))

(event Input|KeyboardEvents|DebugKeyU
  (params (Key :type Key%20Structure :default "None") (ActionValue :type Input%20Action%20Value%20Structure))
  (:Pressed
    (Class|BaseCharacter|LoadGameLocally)
    (Development|PrintString "Loaded Slot 0")))

(event Input|KeyboardEvents|DebugKeyL
  (params (Key :type Key%20Structure :default "None") (ActionValue :type Input%20Action%20Value%20Structure))
  (:Pressed
    (Class|BaseCharacter|LoadGameGlobally)
    (Development|PrintString "GAME LOADED")))

(event Input|KeyboardEvents|DebugKeyK
  (params (Key :type Key%20Structure :default "None") (ActionValue :type Input%20Action%20Value%20Structure))
  (:Pressed
    (Class|BaseCharacter|SaveGameGlobally)
    (Development|PrintString "GAME SAVED")))

(fn ConstructionScript)